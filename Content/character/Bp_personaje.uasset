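; Player character for a 2D side-scroller, handling movement, jump, dash, run and crouch through Enhanced Input.
; Movement runs along world X and flips control rotation yaw to face the travel direction.
; Dash launches the character using half its X velocity, gated by a DoOnce that resets one second after release.
; Input events swap flipbooks directly; run and crouch only change animation, and some run and double-jump nodes are disconnected.
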(event `self.ReceiveBeginPlay`
  (bind _asplayer_controller (cast `PlayerController` (`self.GetController`)))
  (`EnhancedInputSubsystemInterface.AddMappingContext` (pcsubsystem `EnhancedInputLocalPlayerSubsystem` _asplayer_controller) "/Game/character/imput/mca.mca" 0 (struct)))

(event `EnhancedInput|/Game/character/imput/action/IA_saltar`
  (params (ActionValue :type Boolean) (ElapsedSeconds :type "Float (double-precision)") (TriggeredSeconds :type "Float (double-precision)") (InputAction :type "InputAction Object Reference" :default "/Game/character/imput/action/IA_saltar.IA_saltar"))
  ;[1 1 1] Salto y Doble Salto
  (:`Started`
    (`self.Jump`)
    (`PaperFlipbookComponent.SetFlipbook` (`self.Sprite`) "/Game/character/Animation/Jump/Fl_jump.Fl_jump"))
  (:`Completed`
    (`self.StopJumping`)
    (`PaperFlipbookComponent.SetFlipbook` (`self.Sprite`) "/Game/character/Animation/Idle/FL_Idle.FL_Idle")))

(event `EnhancedInput|/Game/character/imput/action/IA_movimiento`
  (params (ActionValue :type "Float (double-precision)") (ElapsedSeconds :type "Float (double-precision)") (TriggeredSeconds :type "Float (double-precision)") (InputAction :type "InputAction Object Reference" :default "/Game/character/imput/action/IA_movimiento.IA_movimiento"))
  ;[1 1 1] Moviemiento
  (:`Triggered`
    (`self.AddMovementInput` (1.0 0.0 0.0) ActionValue)
    (`Controller.SetControlRotation` (`self.GetController`) (select `bool` (> ActionValue 0.0) :`false` (`KismetMathLibrary.MakeRotator` 0.0 0.0 -180.0) :`true` (`KismetMathLibrary.MakeRotator` 0.0))))
  (:`Started`
    (`PaperFlipbookComponent.SetFlipbook` (`self.Sprite`) "/Game/character/Animation/Walk/FL_walk.FL_walk"))
  (:`Completed`
    (`PaperFlipbookComponent.SetFlipbook` (`self.Sprite`) "/Game/character/Animation/Idle/FL_Idle.FL_Idle")))

(event `EnhancedInput|/Game/character/imput/action/IA_Dash`
  (params (ActionValue :type "Float (double-precision)") (ElapsedSeconds :type "Float (double-precision)") (TriggeredSeconds :type "Float (double-precision)") (InputAction :type "InputAction Object Reference" :default "/Game/character/imput/action/IA_Dash.IA_Dash"))
  (bind _returnvalue_x (`KismetMathLibrary.BreakVector` (* (`self.GetVelocity`) 0.5)))
  ;[1 1 1] Dash
  (:`Started`
    (`/Engine/EditorBlueprintResources/StandardMacros.DoOnce` false :!label _label
      (:`Completed`
        (`PaperFlipbookComponent.SetFlipbook` (`self.Sprite`) "/Game/character/Animation/Dash/FL_dash.FL_dash")
        (`self.LaunchCharacter` (`KismetMathLibrary.MakeVector` _returnvalue_x 0.0 1.0)))))
  (:`Completed`
    (`KismetSystemLibrary.Delay` 1.0)
    (goto _label :!via `Reset`)))

(event `EnhancedInput|/Game/character/imput/action/IA_Run`
  (params (ActionValue :type "Float (double-precision)") (ElapsedSeconds :type "Float (double-precision)") (TriggeredSeconds :type "Float (double-precision)") (InputAction :type "InputAction Object Reference" :default "/Game/character/imput/action/IA_Run.IA_Run"))
  ;[1 1 1] run
  (:`Started`
    (`PaperFlipbookComponent.SetFlipbook` (`self.Sprite`) "/Game/character/Animation/Run/Fl_Run.Fl_Run"))
  (:`Completed`
    (`PaperFlipbookComponent.SetFlipbook` (`self.Sprite`) "/Game/character/Animation/Idle/FL_Idle.FL_Idle")))

(event `EnhancedInput|/Game/character/imput/action/IA_crown`
  (params (ActionValue :type "Float (double-precision)") (ElapsedSeconds :type "Float (double-precision)") (TriggeredSeconds :type "Float (double-precision)") (InputAction :type "InputAction Object Reference" :default "/Game/character/imput/action/IA_crown.IA_crown"))
  ;[1 1 1] agacharse
  (:`Started`
    (`PaperFlipbookComponent.SetFlipbook` (`self.Sprite`) "/Game/character/Animation/Crown/FL_crown.FL_crown"))
  (:`Completed`
    (`PaperFlipbookComponent.SetFlipbook` (`self.Sprite`) "/Game/character/Animation/Idle/FL_Idle.FL_Idle")))

(fn `UserConstructionScript`)