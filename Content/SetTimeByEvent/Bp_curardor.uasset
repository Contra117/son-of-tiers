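; Healer test Blueprint that periodically restores its own health variable (Vida) up to a maximum (VidaMax).
; BeginPlay starts a looping event timer at the TicksCuracion interval, firing a custom event that adds a fixed amount and prints the new value.
; At maximum, it tries to clear the timer by the name "curar personaje" rather than a stored handle, and prints a debug message.
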(event `self.ReceiveBeginPlay`
  (`KismetSystemLibrary.K2_SetTimerDelegate` (delegate `curar personaje`) (`self.TicksCuracion`) true)
  (`KismetSystemLibrary.PrintString` "aca sige" true true (struct :`R` 1.0 :`B` 0.015653 :`A` 1.0) 60.0))

(event `curar personaje`
  (if (>= (`self.vida`) (`self.VidaMax`))
    (`KismetSystemLibrary.K2_ClearTimer` null "curar personaje")
    (`KismetSystemLibrary.PrintString` "esto se limpio")
    (else
      (bind _output_get (set `self.vida` (+ (`self.vida`) 10.0)))
      (`KismetSystemLibrary.PrintString` (`KismetStringLibrary.Concat_StrStr` "a curado el pj \n" (`KismetStringLibrary.Conv_DoubleToString` _output_get)) true true (struct :`G` 0.66 :`B` 1.0 :`A` 1.0) 5.0))))

(fn `UserConstructionScript`)